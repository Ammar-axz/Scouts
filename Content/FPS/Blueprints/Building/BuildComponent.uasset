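; Building component for the first-person character that previews and places structures from a data table at a Wood cost.
; A looping delayed camera multi-trace drives a green or red ghost mesh showing placement validity.
; Foundations sit on landscape, while pieces snap to building components whose tags match the build ID.
; Spawning links to the parent building, disables the used socket's collision and records the piece in GM_EditMap when present.
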(event Custom|StopBuild
  (bind _ghostbuild (Variables|Default|GetGhostBuild))
  (Utilities|IsValid _ghostbuild
    (:Is%20Valid
      (Default|DestroyComponent (Variables|Default|GetAs%20FPSArms%20Character) _ghostbuild))))

(event Custom|BuildDelay
  (bind _as_fpsarms_character (Variables|Default|GetAs%20FPSArms%20Character))
  (bind _buildid (Variables|Default|GetBuildId))
  (bind _firstpersoncamera (Variables|/Game/FPS/Blueprints/FPSArms_character.FPSArms_character_C|GetFirstPersonCamera _as_fpsarms_character))
  (bind _returnvalue (Transformation|GetWorldLocation _firstpersoncamera))
  (bind _returnvalue_2 (Math|Vector|GetForwardVector _firstpersoncamera))
  (bind _returnvalue_3 (* _returnvalue_2 5e+02))
  (bind _returnvalue_4 (+ _returnvalue _returnvalue_3))
  (Utilities|FlowControl|Delay 0.2)
  (Utilities|IsValid _as_fpsarms_character
    (:Is%20Valid
      (Variables|Default|SetBuildIdChange (== _buildid (Variables|Default|GetCurrentBuildId)))
      (if (== _buildid (Variables|Default|GetCurrentBuildId))
        _
        (else
          (Variables|Default|SetCurrentBuildId _buildid)
          (CallFunction|ChangeBuildable)))
      (bind (_outhits _returnvalue_5) (Collision|MultiLineTraceByChannel (+ _returnvalue (* _returnvalue_2 1e+02)) _returnvalue_4 "TraceTypeQuery1" false 0 "ForDuration" true "(R=1.000000,G=0.000000,B=0.000000,A=1.000000)" "(R=0.000000,G=1.000000,B=0.000000,A=1.000000)" 2.0))
      (Variables|Default|SetTraceMatchFlag false)
      (Variables|Default|SetHit%20Component 0)
      (bind _array_element (Utilities|Array|ForEachLoopwithBreak _outhits :!label _label)
        (:LoopBody
          (if (Variables|Default|GetTraceMatchFlag)
            (goto _label Break)
            (else
              (bind _output_get (Variables|Default|SetHit%20Component (.HitComponent (Collision|BreakHitResult _array_element))))
              (Utilities|Casting|CastToBuildingBase (.HitActor (Collision|BreakHitResult _array_element)))
              (bind _array_element_2 (Utilities|Array|ForEachLoopwithBreak (Variables|/Script/Engine.ActorComponent|GetComponentTags _output_get) :!label _label_2)
                (:LoopBody
                  (if (Utilities|Enum|Equal(Enum) (Utilities|String|ToString(Name) _array_element_2) (Utilities|String|ToString(Integer) (Variables|Default|GetBuildId)))
                    (Variables|Default|SetMatchTrace _array_element)
                    (Variables|Default|SetTraceMatchFlag true)
                    (goto _label_2 Break)
                    (else
                      (Variables|Default|SetTraceMatchFlag false))))))))
        (:Completed
          (if (== (.HitComponent (Collision|BreakHitResult (select (Variables|Default|GetTraceMatchFlag) (Variables|Default|GetMatchTrace) _array_element))) (Variables|Default|GetHit%20Component))
            (if (Variables|Default|GetBuildIdChange)
              (if (Class|KismetMathLibrary|EqualExactlyVectorVector (Variables|Default|GetImpact%20Point) (.ImpactPoint (Collision|BreakHitResult (select (Variables|Default|GetTraceMatchFlag) (Variables|Default|GetMatchTrace) _array_element))))
                _
                (else
                  (Variables|Default|SetImpact%20Point (.ImpactPoint (Collision|BreakHitResult (select (Variables|Default|GetTraceMatchFlag) (Variables|Default|GetMatchTrace) _array_element))))
                  (CallFunction|SpawnBuildGhost (select (Variables|Default|GetTraceMatchFlag) (Variables|Default|GetMatchTrace) _array_element) _returnvalue_5 _returnvalue_4 :!label _label_3)))
              (else
                (goto _label_3)))
            (else
              (goto _label_3)))
          (CallFunction|BuildDelay))))))

(event Custom|StartBuild
  (bind _as_fpsarms_character (Variables|Default|GetAs%20FPSArms%20Character))
  (bind _buildid (Variables|Default|GetBuildId))
  (bind _firstpersoncamera (Variables|/Game/FPS/Blueprints/FPSArms_character.FPSArms_character_C|GetFirstPersonCamera _as_fpsarms_character))
  (bind _returnvalue (Transformation|GetWorldLocation _firstpersoncamera))
  (bind _returnvalue_2 (Math|Vector|GetForwardVector _firstpersoncamera))
  (bind _returnvalue_3 (* _returnvalue_2 5e+02))
  (bind _returnvalue_4 (+ _returnvalue _returnvalue_3))
  (Utilities|IsValid _as_fpsarms_character
    (:Is%20Valid
      (Variables|Default|SetBuildIdChange (== _buildid (Variables|Default|GetCurrentBuildId)))
      (if (== _buildid (Variables|Default|GetCurrentBuildId))
        _
        (else
          (Variables|Default|SetCurrentBuildId _buildid)
          (CallFunction|ChangeBuildable)))
      (bind (_outhits _returnvalue_5) (Collision|MultiLineTraceByChannel (+ _returnvalue (* _returnvalue_2 1e+02)) _returnvalue_4 "TraceTypeQuery1" false 0 "ForDuration" true "(R=1.000000,G=0.000000,B=0.000000,A=1.000000)" "(R=0.000000,G=1.000000,B=0.000000,A=1.000000)" 2.0))
      (Variables|Default|SetTraceMatchFlag false)
      (Variables|Default|SetHit%20Component 0)
      (bind _array_element (Utilities|Array|ForEachLoopwithBreak _outhits :!label _label)
        (:LoopBody
          (if (Variables|Default|GetTraceMatchFlag)
            (goto _label Break)
            (else
              (bind _output_get (Variables|Default|SetHit%20Component (.HitComponent (Collision|BreakHitResult _array_element))))
              (Utilities|Casting|CastToBuildingBase (.HitActor (Collision|BreakHitResult _array_element)))
              (bind _array_element_2 (Utilities|Array|ForEachLoopwithBreak (Variables|/Script/Engine.ActorComponent|GetComponentTags _output_get) :!label _label_2)
                (:LoopBody
                  (if (Utilities|Enum|Equal(Enum) (Utilities|String|ToString(Name) _array_element_2) (Utilities|String|ToString(Integer) (Variables|Default|GetBuildId)))
                    (Variables|Default|SetMatchTrace _array_element)
                    (Variables|Default|SetTraceMatchFlag true)
                    (goto _label_2 Break)
                    (else
                      (Variables|Default|SetTraceMatchFlag false))))))))
        (:Completed
          (if (== (.HitComponent (Collision|BreakHitResult (select (Variables|Default|GetTraceMatchFlag) (Variables|Default|GetMatchTrace) _array_element))) (Variables|Default|GetHit%20Component))
            (if (Variables|Default|GetBuildIdChange)
              (if (Class|KismetMathLibrary|EqualExactlyVectorVector (Variables|Default|GetImpact%20Point) (.ImpactPoint (Collision|BreakHitResult (select (Variables|Default|GetTraceMatchFlag) (Variables|Default|GetMatchTrace) _array_element))))
                _
                (else
                  (Variables|Default|SetImpact%20Point (.ImpactPoint (Collision|BreakHitResult (select (Variables|Default|GetTraceMatchFlag) (Variables|Default|GetMatchTrace) _array_element))))
                  (CallFunction|SpawnBuildGhost (select (Variables|Default|GetTraceMatchFlag) (Variables|Default|GetMatchTrace) _array_element) _returnvalue_5 _returnvalue_4 :!label _label_3)))
              (else
                (goto _label_3)))
            (else
              (goto _label_3)))
          (CallFunction|BuildDelay))))))

(event EventTick
  (params (DeltaSeconds :type Float%20%28single-precision%29))
  (Development|PrintString (Utilities|GetDisplayName (Variables|Default|GetHit%20Component)) true true "(R=0.000000,G=0.660000,B=1.000000,A=1.000000)" DeltaSeconds))

(event EventBeginPlay
  (bind _asfpsarms_character (Utilities|Casting|CastToFPSArms_character (Game|GetPlayerCharacter 0)))
  (Variables|Default|SetAs%20FPSArms%20Character _asfpsarms_character)
  (bind _outrownames (DataTable|GetDataTableRowNames "/Game/FPS/Blueprints/Building/BuildablesDB.BuildablesDB"))
  (for _array_element _outrownames
    (bind _returnvalue (Utilities|GetDataTableRow "/Game/FPS/Blueprints/Building/BuildablesDB.BuildablesDB" _array_element)
      (:then
        (Utilities|Array|Add (Variables|Default|GetBuildables) _returnvalue)
        (bind _asgm_edit_map (Utilities|Casting|CastToGM_EditMap (Game|GetGameMode)))
        (Variables|Default|SetAs%20GM%20Edit%20Map _asgm_edit_map)))))

(fn SpawnBuildGhost
  (params (HitResult :type Hit%20Result%20Structure) (ReturnValue :type Boolean) (TraceEnd :type Vector))
  (bind (_bblockinghit _binitialoverlap _time _distance _location _impactpoint _normal _impactnormal _physmat _hitactor _hitcomponent _hitbonename _bonename _hititem _elementindex _faceindex _tracestart _traceend) (Collision|BreakHitResult HitResult))
  (bind _as_fpsarms_character (Variables|Default|GetAs%20FPSArms%20Character))
  (bind _firstpersoncamera (Variables|/Game/FPS/Blueprints/FPSArms_character.FPSArms_character_C|GetFirstPersonCamera _as_fpsarms_character))
  (bind _returnvalue (Transformation|GetWorldRotation _firstpersoncamera))
  (bind _returnvalue_2 (Math|Rotator|MakeRotator 0.0 0.0 (.yaw _returnvalue)))
  (Development|PrintString (Utilities|String|ToString(Boolean) (Variables|Default|GetTraceMatchFlag)))
  (if ReturnValue
    (Variables|Default|SetSpawnTransform (Math|Transform|MakeTransform _impactpoint _returnvalue_2 "1.000000,1.000000,1.000000") :!label _label)
    (Variables|Default|SetHit%20Actor _hitactor)
    (bind _asbuilding_base (Utilities|Casting|CastToBuildingBase _hitactor)
      (:then
        (Variables|Default|SetLast%20Hit%20Building _asbuilding_base))
      (:CastFailed
        _))
    (if (Variables|Default|GetGhostSpawned)
      (bind _spawntransform (CallFunction|DetectSnappingBox2 _hitcomponent (Math|Transform|MakeTransform _traceend _returnvalue_2)))
      (if (Variables|Default|GetCanBuild)
        (Transformation|DetachFromComponent (Variables|/Script/Engine.Actor|GetRootComponent (Variables|Default|GetGhostBuild)) "KeepRelative" "KeepRelative" "KeepRelative" true)
        (else
          (Transformation|AttachComponentToComponent (Variables|/Script/Engine.Actor|GetRootComponent (Variables|Default|GetGhostBuild)) (Variables|/Game/FPS/Blueprints/FPSArms_character.FPSArms_character_C|GetFirstPersonCamera (Variables|Default|GetAs%20FPSArms%20Character)) "None" "SnapToTarget" "SnapToTarget" "SnapToTarget" true)))
      (CallFunction|UpdatePosition _spawntransform)
      (else
        (bind _ghostbuildref (Default|AttachBuildGhosttoCharacter (Variables|Default|GetAs%20FPSArms%20Character) (Variables|Default|GetSpawnTransform) :!label _label_2))
        (Variables|Default|SetGhostBuild _ghostbuildref)
        (Components|StaticMesh|SetStaticMesh (Variables|/Game/FPS/Blueprints/Building/BP_GhostBuild.BP_GhostBuild_C|GetStaticMesh (Variables|Default|GetGhostBuild)) (.mesh (Utilities|Array|Get(acopy) (Variables|Default|GetBuildables) (Variables|Default|GetCurrentBuildId))))
        (Collision|SetCollisionEnabled (Variables|/Game/FPS/Blueprints/Building/BP_GhostBuild.BP_GhostBuild_C|GetStaticMesh (Variables|Default|GetGhostBuild)) "NoCollision")
        (Variables|Default|SetGhostSpawned true)))
    (elif (Variables|Default|GetTraceMatchFlag)
      (goto _label)
      (else
        (Variables|Default|SetCanBuild false)
        (Variables|Default|SetSpawnTransform (Math|Transform|MakeTransform TraceEnd _returnvalue_2 "1.000000,1.000000,1.000000"))
        (Variables|Default|SetHit%20Actor 0)
        (if (Variables|Default|GetGhostSpawned)
          (Transformation|AttachComponentToComponent (Variables|/Script/Engine.Actor|GetRootComponent (Variables|Default|GetGhostBuild)) (Variables|/Game/FPS/Blueprints/FPSArms_character.FPSArms_character_C|GetFirstPersonCamera (Variables|Default|GetAs%20FPSArms%20Character)) "None" "SnapToTarget" "SnapToTarget" "SnapToTarget" true)
          (CallFunction|UpdatePosition (Variables|Default|GetSpawnTransform))
          (else
            (goto _label_2))))))
  (CallFunction|BuildGhostColor)
  (return))

(fn UpdatePosition
  (params (Transform :type Transform%20%28by%20ref%29))
  (Transformation|SetWorldTransform (Variables|/Script/Engine.Actor|GetRootComponent (Variables|Default|GetGhostBuild)) Transform true false))

(fn ChangeBuildable
  (Components|StaticMesh|SetStaticMesh (Variables|/Game/FPS/Blueprints/Building/BP_GhostBuild.BP_GhostBuild_C|GetStaticMesh (Variables|Default|GetGhostBuild)) (.mesh (Utilities|Array|Get(acopy) (Variables|Default|GetBuildables) (Variables|Default|GetCurrentBuildId)))))

(fn SpawnBuild
  (bind _buildables (Variables|Default|GetBuildables))
  (bind _currentbuildid (Variables|Default|GetCurrentBuildId))
  (bind _as_gm_edit_map (Variables|Default|GetAs%20GM%20Edit%20Map))
  (bind _ghostbuild (Variables|Default|GetGhostBuild))
  (bind _currentbuildid_2 (Variables|Default|GetCurrentBuildId))
  (bind _buildables_2 (Variables|Default|GetBuildables))
  (bind _hit_component (Variables|Default|GetHit%20Component))
  (bind _as_fpsarms_character (Variables|Default|GetAs%20FPSArms%20Character))
  (bind _output (Utilities|Array|Get(acopy) _buildables _currentbuildid))
  (bind _output_2 (Utilities|Array|Get(acopy) _buildables_2 _currentbuildid_2))
  (Utilities|IsValid _ghostbuild
    (:Is%20Valid
      (if (Variables|Default|GetCanBuild)
        (if (>= (Variables|/Game/FPS/Blueprints/FPSArms_character.FPSArms_character_C|GetWood (Variables|Default|GetAs%20FPSArms%20Character)) (.wood _output_2))
          (bind _returnvalue (Game|SpawnActorfromClass (.actor _output_2) (Transformation|GetWorldTransform (Variables|/Script/Engine.Actor|GetRootComponent _ghostbuild)) "Undefined" "SelectDefaultAtRuntime" 0 0))
          (bind _asbuilding_base (Utilities|Casting|CastToBuildingBase (Variables|Default|GetHit%20Actor))
            (:then
              (bind _asbuilding_base_2 (Utilities|Casting|CastToBuildingBase _returnvalue))
              (Default|SetParentBuildandCollision _asbuilding_base_2 _asbuilding_base _hit_component)
              (Collision|SetCollisionEnabled _hit_component "NoCollision"))
            (:CastFailed
              _))
          (Variables|/Game/FPS/Blueprints/FPSArms_character.FPSArms_character_C|SetWood _as_fpsarms_character (- (Variables|/Game/FPS/Blueprints/FPSArms_character.FPSArms_character_C|GetWood _as_fpsarms_character) (.wood _output_2)))
          (Utilities|IsValid _as_gm_edit_map
            (:Is%20Valid
              (bind _result (Math|Integer|IncrementInt (Variables|/Game/FPS/Blueprints/GameMode/GM_EditMap.GM_EditMap_C|GetIndex _as_gm_edit_map))
                (:%20%20
                  (Class|BPIBuilding|AddIndex(Message) _asbuilding_base _result)
                  (Default|AddActor _as_gm_edit_map (Utilities|Struct|MakeStruct_MapSave _result (.actor _output) (.mesh _output) (Transformation|GetWorldTransform (Variables|/Script/Engine.Actor|GetRootComponent (Variables|Default|GetGhostBuild))) (.wood _output)))
                  (Development|PrintString (Utilities|String|ToString(Integer) _result)))))))))))

(fn BuildGhostColor
  (bind _ghostbuild (Variables|Default|GetGhostBuild))
  (bind _staticmesh (Variables|/Game/FPS/Blueprints/Building/BP_GhostBuild.BP_GhostBuild_C|GetStaticMesh _ghostbuild))
  ;[1 1 1] for loop to iterate through all the materials on the ghost build mesh
  (for _index (range 0 (- (Rendering|Material|GetNumMaterials (Variables|/Game/FPS/Blueprints/Building/BP_GhostBuild.BP_GhostBuild_C|GetStaticMesh (Variables|Default|GetGhostBuild))) 1))
    (if (Variables|Default|GetCanBuild)
      (Rendering|Material|SetMaterial _staticmesh _index "/Game/FPS/Blueprints/Building/GhostGreen.GhostGreen")
      (else
        (Rendering|Material|SetMaterial _staticmesh _index "/Game/FPS/Blueprints/Building/GhostRed.GhostRed")))))

(fn DetectSnappingBox2
  (params (HitComponent :type Primitive%20Component%20Object%20Reference) (TraceEnd :type Transform))
  (bind _ghostbuild (Variables|Default|GetGhostBuild))
  (bind _hit_actor (Variables|Default|GetHit%20Actor))
  (bind _spawntransform (Variables|Default|GetSpawnTransform))
  (bind _buildid (Variables|Default|GetBuildId))
  (bind _returnvalue (Utilities|String|ToString(Integer) _buildid))
  (bind _staticmesh (Variables|/Game/FPS/Blueprints/Building/BP_GhostBuild.BP_GhostBuild_C|GetStaticMesh _ghostbuild))
  (bind _staticmesh_2 (Variables|/Script/Engine.StaticMeshComponent|GetStaticMesh _staticmesh))
  (Utilities|Casting|CastToLandscape _hit_actor
    (:then
      (if (or (== _staticmesh_2 "/Game/FPS/Blueprints/Building/BuildMeshes/Foundation.Foundation") (== _staticmesh_2 "/Game/FPS/Blueprints/Building/BuildMeshes/FoundationTriangle.FoundationTriangle"))
        (LocalVariables|SetSelectTransform _spawntransform)
        (Variables|Default|SetCanBuild true :!label _label)
        (else
          (LocalVariables|SetSelectTransform _spawntransform :!label _label_2)
          (Variables|Default|SetCanBuild false :!label _label_3)))
      (return (LocalVariables|GetSelectTransform)))
    (:CastFailed
      (Utilities|Casting|CastToBuildingBase _hit_actor
        (:then
          (bind _output_get (Variables|Default|SetHit%20Component HitComponent))
          (bind _array_element (Utilities|Array|ForEachLoopwithBreak (Variables|/Script/Engine.ActorComponent|GetComponentTags _output_get) :!label _label_4)
            (:LoopBody
              (if (Utilities|Enum|Equal(Enum) (Utilities|String|ToString(Name) _array_element) _returnvalue)
                (LocalVariables|SetMatchType _array_element)
                (goto _label_4 Break)))
            (:Completed
              (if (Utilities|Enum|Equal(Enum) (Utilities|String|ToString(Name) (LocalVariables|GetMatchType)) _returnvalue)
                (LocalVariables|SetSelectTransform (Transformation|GetWorldTransform (Variables|Default|GetHit%20Component)))
                (goto _label)
                (else
                  (LocalVariables|SetSelectTransform TraceEnd)
                  (goto _label_3))))))
        (:CastFailed
          (goto _label_2))))))