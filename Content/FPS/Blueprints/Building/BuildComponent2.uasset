(event Custom|GhostBeginOverlap
  (params (OverlappedComponent :type Primitive%20Component%20Object%20Reference) (OtherActor :type Actor%20Object%20Reference) (OtherComp :type Primitive%20Component%20Object%20Reference) (OtherBodyIndex :type Integer) (bFromSweep :type Boolean) (SweepResult :type Hit%20Result%20Structure%20%28by%20ref%29))
  (Development|PrintString (Utilities|GetDisplayName OtherComp)))

(event Custom|StopBuild
  (bind _ghostbuild (Variables|Default|GetGhostBuild))
  (Utilities|IsValid _ghostbuild
    (:Is%20Valid
      (Default|DestroyComponent (Variables|Default|GetAs%20FPSArms%20Character) (Variables|/Script/Engine.Actor|GetRootComponent _ghostbuild)))))

(event Custom|SphereCollisionBeginOverlap2
  (params (OverlappedComponent :type Primitive%20Component%20Object%20Reference) (OtherActor :type Actor%20Object%20Reference) (OtherComp :type Primitive%20Component%20Object%20Reference) (OtherBodyIndex :type Integer) (bFromSweep :type Boolean) (SweepResult :type Hit%20Result%20Structure%20%28by%20ref%29)))

(event Custom|BuildDelay
  (bind _as_fpsarms_character (Variables|Default|GetAs%20FPSArms%20Character))
  (bind _buildid (Variables|Default|GetBuildId))
  (bind _firstpersoncamera (Variables|/Game/FPS/Blueprints/FPSArms_character.FPSArms_character_C|GetFirstPersonCamera _as_fpsarms_character))
  (bind _returnvalue (Transformation|GetWorldLocation _firstpersoncamera))
  (bind _returnvalue_2 (Math|Vector|GetForwardVector _firstpersoncamera))
  (Utilities|FlowControl|Delay 0.2)
  (Utilities|IsValid _as_fpsarms_character
    (:Is%20Valid
      (Variables|Default|SetBuildIdChange (== _buildid (Variables|Default|GetCurrentBuildId)))
      (if (== _buildid (Variables|Default|GetCurrentBuildId))
        _
        (else
          (Variables|Default|SetCurrentBuildId _buildid)
          (CallFunction|DisableAllSnappinginBuild)
          (CallFunction|ChangeBuildable)))
      (bind (_outhit _returnvalue_3) (Collision|LineTraceByChannel (+ _returnvalue (* _returnvalue_2 1e+02)) (+ _returnvalue (* _returnvalue_2 5e+02)) "TraceTypeQuery1" false 0 "ForOneFrame"))
      (if (Variables|Default|GetBuildIdChange)
        (if (Class|KismetMathLibrary|EqualExactlyVectorVector (Variables|Default|GetImpact%20Point) (.ImpactPoint (Collision|BreakHitResult _outhit)))
          _
          (else
            (Variables|Default|SetImpact%20Point (.ImpactPoint (Collision|BreakHitResult _outhit)))
            (Utilities|Casting|CastToBuildingBase (.HitActor (Collision|BreakHitResult _outhit))
              (:then
                (if (== (.HitComponent (Collision|BreakHitResult _outhit)) (Variables|Default|GetHit%20Component))
                  _
                  (else
                    (CallFunction|SpawnBuildGhost _outhit _returnvalue_3 :!label _label))))
              (:CastFailed
                (goto _label)))))
        (else
          (goto _label)))
      (CallFunction|BuildDelay))))

(event Custom|StartBuild
  (bind _as_fpsarms_character (Variables|Default|GetAs%20FPSArms%20Character))
  (bind _buildid (Variables|Default|GetBuildId))
  (bind _firstpersoncamera (Variables|/Game/FPS/Blueprints/FPSArms_character.FPSArms_character_C|GetFirstPersonCamera _as_fpsarms_character))
  (bind _returnvalue (Transformation|GetWorldLocation _firstpersoncamera))
  (bind _returnvalue_2 (Math|Vector|GetForwardVector _firstpersoncamera))
  (Utilities|IsValid _as_fpsarms_character
    (:Is%20Valid
      (Variables|Default|SetBuildIdChange (== _buildid (Variables|Default|GetCurrentBuildId)))
      (if (== _buildid (Variables|Default|GetCurrentBuildId))
        _
        (else
          (Variables|Default|SetCurrentBuildId _buildid)
          (CallFunction|DisableAllSnappinginBuild)
          (CallFunction|ChangeBuildable)))
      (bind (_outhit _returnvalue_3) (Collision|LineTraceByChannel (+ _returnvalue (* _returnvalue_2 1e+02)) (+ _returnvalue (* _returnvalue_2 5e+02)) "TraceTypeQuery1" false 0 "ForOneFrame"))
      (if (Variables|Default|GetBuildIdChange)
        (if (Class|KismetMathLibrary|EqualExactlyVectorVector (Variables|Default|GetImpact%20Point) (.ImpactPoint (Collision|BreakHitResult _outhit)))
          _
          (else
            (Variables|Default|SetImpact%20Point (.ImpactPoint (Collision|BreakHitResult _outhit)))
            (Utilities|Casting|CastToBuildingBase (.HitActor (Collision|BreakHitResult _outhit))
              (:then
                (if (== (.HitComponent (Collision|BreakHitResult _outhit)) (Variables|Default|GetHit%20Component))
                  _
                  (else
                    (CallFunction|SpawnBuildGhost _outhit _returnvalue_3 :!label _label))))
              (:CastFailed
                (goto _label)))))
        (else
          (goto _label)))
      (CallFunction|BuildDelay))))

(event Custom|SphereCollisionOnEndOverlap
  (params (OverlappedComponent :type Primitive%20Component%20Object%20Reference) (OtherActor :type Actor%20Object%20Reference) (OtherComp :type Primitive%20Component%20Object%20Reference) (OtherBodyIndex :type Integer)))

(event Custom|SphereCollisionBeginOverlap
  (params (OverlappedComponent :type Primitive%20Component%20Object%20Reference) (OtherActor :type Actor%20Object%20Reference) (OtherComp :type Primitive%20Component%20Object%20Reference) (OtherBodyIndex :type Integer) (bFromSweep :type Boolean) (SweepResult :type Hit%20Result%20Structure%20%28by%20ref%29))
  (bind _returnvalue (Utilities|GetDisplayName OtherComp))
  (bind _returnvalue_2 (Utilities|String|FindSubstring _returnvalue "."))
  (bind _returnvalue_3 (+ _returnvalue_2 1))
  (bind _returnvalue_4 (Utilities|String|GetSubstring _returnvalue _returnvalue_3 20))
  ;[1 1 1] Get the Overlapping snapping box name
  (Utilities|Casting|CastToBuildingBase OtherActor)
  (bind _index (Utilities|FlowControl|ForLoopwithBreak 1 4 :!label _label)
    (:LoopBody
      (if (!= (Utilities|String|FindSubstring _returnvalue_4 (Utilities|String|ToString(Integer) _index)) -1)
        (goto _label Break)
        (else
          (Variables|Default|SetNewVar ""))))
    (:Completed
      (bind _returnvalue_5 (Utilities|GetDataTableRow "/Game/FPS/Blueprints/Building/BuildablesDB.BuildablesDB" (Utilities|String|StringToName (Utilities|String|GetSubstring _returnvalue_4 0 (Utilities|String|FindSubstring _returnvalue_4 (Utilities|String|ToString(Integer) _index)))))
        (:then
          (if (== (.Type (Utilities|Struct|BreakS_Buildables _returnvalue_5)) (.type (Utilities|Array|Get(acopy) (Variables|Default|GetBuildables) (Variables|Default|GetCurrentBuildId))))
            (bind _output_get (Variables|Default|SetNewVar (Utilities|String|Append (Utilities|String|GetSubstring _returnvalue_4 0 (Utilities|String|FindSubstring _returnvalue_4 (Utilities|String|ToString(Integer) _index))) "<<<-----")))
            (Development|PrintString _output_get)))))))

(event EventTick
  (params (DeltaSeconds :type Float%20%28single-precision%29)))

(event EventBeginPlay
  (bind _asfpsarms_character (Utilities|Casting|CastToFPSArms_character (Game|GetPlayerCharacter 0)))
  (Variables|Default|SetAs%20FPSArms%20Character _asfpsarms_character)
  (bind _outrownames (DataTable|GetDataTableRowNames "/Game/FPS/Blueprints/Building/BuildablesDB.BuildablesDB"))
  (for _array_element _outrownames
    (bind _returnvalue (Utilities|GetDataTableRow "/Game/FPS/Blueprints/Building/BuildablesDB.BuildablesDB" _array_element)
      (:then
        (Utilities|Array|Add (Variables|Default|GetBuildables) _returnvalue)
        (bind _asgm_edit_map (Utilities|Casting|CastToGM_EditMap (Game|GetGameMode)))
        (Variables|Default|SetAs%20GM%20Edit%20Map _asgm_edit_map)))))

(fn SpawnBuildGhost
  (params (HitResult :type Hit%20Result%20Structure) (ReturnValue :type Boolean))
  (bind (_bblockinghit _binitialoverlap _time _distance _location _impactpoint _normal _impactnormal _physmat _hitactor _hitcomponent _hitbonename _bonename _hititem _elementindex _faceindex _tracestart _traceend) (Collision|BreakHitResult HitResult))
  (bind _as_fpsarms_character (Variables|Default|GetAs%20FPSArms%20Character))
  (bind _firstpersoncamera (Variables|/Game/FPS/Blueprints/FPSArms_character.FPSArms_character_C|GetFirstPersonCamera _as_fpsarms_character))
  (bind _returnvalue (Transformation|GetWorldRotation _firstpersoncamera))
  (bind _returnvalue_2 (Math|Rotator|MakeRotator 0.0 0.0 (.yaw _returnvalue)))
  (if ReturnValue
    (Variables|Default|SetSpawnTransform (Math|Transform|MakeTransform _impactpoint _returnvalue_2 "1.000000,1.000000,1.000000"))
    (if (== (Variables|Default|GetHit%20Actor) _hitactor)
      _
      (else
        (CallFunction|DisableAllSnappinginBuild)))
    (Variables|Default|SetHit%20Actor _hitactor)
    (Variables|Default|SetHit%20Component _hitcomponent)
    (bind _asbuilding_base (Utilities|Casting|CastToBuildingBase _hitactor)
      (:then
        (Variables|Default|SetLast%20Hit%20Building _asbuilding_base))
      (:CastFailed
        _))
    (if (Variables|Default|GetGhostSpawned)
      (CallFunction|DetectSnappingBox)
      (bind _transform (CallFunction|BuildOnlyonSnapping))
      (Transformation|DetachFromComponent (Variables|/Script/Engine.Actor|GetRootComponent (Variables|Default|GetGhostBuild)) "KeepRelative" "KeepRelative" "KeepRelative" true)
      (CallFunction|UpdatePosition (select (Variables|Default|GetCanBuild) _transform (Variables|Default|GetSpawnTransform)))
      (else
        (bind _ghostbuildref (Default|AttachBuildGhosttoCharacter (Variables|Default|GetAs%20FPSArms%20Character) (Variables|Default|GetSpawnTransform) :!label _label))
        (Variables|Default|SetGhostBuild _ghostbuildref)
        (Components|StaticMesh|SetStaticMesh (Variables|/Game/FPS/Blueprints/Building/BP_GhostBuild.BP_GhostBuild_C|GetStaticMesh (Variables|Default|GetGhostBuild)) (.mesh (Utilities|Array|Get(acopy) (Variables|Default|GetBuildables) (Variables|Default|GetCurrentBuildId))))
        (Collision|SetCollisionEnabled (Variables|/Game/FPS/Blueprints/Building/BP_GhostBuild.BP_GhostBuild_C|GetStaticMesh (Variables|Default|GetGhostBuild)) "QueryOnly")
        (Variables|Default|SetGhostSpawned true)))
    (else
      (Variables|Default|SetCanBuild false)
      (Variables|Default|SetSpawnTransform (Math|Transform|MakeTransform _traceend _returnvalue_2 "1.000000,1.000000,1.000000"))
      (Variables|Default|SetHit%20Component _hitcomponent)
      (if (Variables|Default|GetGhostSpawned)
        (Transformation|AttachComponentToComponent (Variables|/Script/Engine.Actor|GetRootComponent (Variables|Default|GetGhostBuild)) (Variables|/Game/FPS/Blueprints/FPSArms_character.FPSArms_character_C|GetFirstPersonCamera (Variables|Default|GetAs%20FPSArms%20Character)) "None" "SnapToTarget" "SnapToTarget" "SnapToTarget" true)
        (CallFunction|UpdatePosition (Variables|Default|GetSpawnTransform))
        (else
          (goto _label)))))
  (CallFunction|BuildGhostColor)
  (return))

(fn UpdatePosition
  (params (Transform :type Transform%20%28by%20ref%29))
  (Transformation|SetWorldTransform (Variables|/Script/Engine.Actor|GetRootComponent (Variables|Default|GetGhostBuild)) Transform true false))

(fn ChangeBuildable
  (Components|StaticMesh|SetStaticMesh (Variables|/Game/FPS/Blueprints/Building/BP_GhostBuild.BP_GhostBuild_C|GetStaticMesh (Variables|Default|GetGhostBuild)) (.mesh (Utilities|Array|Get(acopy) (Variables|Default|GetBuildables) (Variables|Default|GetCurrentBuildId)))))

(fn SpawnBuild
  (bind _buildables (Variables|Default|GetBuildables))
  (bind _currentbuildid (Variables|Default|GetCurrentBuildId))
  (bind _as_gm_edit_map (Variables|Default|GetAs%20GM%20Edit%20Map))
  (bind _ghostbuild (Variables|Default|GetGhostBuild))
  (bind _currentbuildid_2 (Variables|Default|GetCurrentBuildId))
  (bind _buildables_2 (Variables|Default|GetBuildables))
  (bind _hit_component (Variables|Default|GetHit%20Component))
  (bind _as_fpsarms_character (Variables|Default|GetAs%20FPSArms%20Character))
  (bind _output (Utilities|Array|Get(acopy) _buildables _currentbuildid))
  (bind _output_2 (Utilities|Array|Get(acopy) _buildables_2 _currentbuildid_2))
  (Utilities|IsValid _ghostbuild
    (:Is%20Valid
      (if (Variables|Default|GetCanBuild)
        (if (>= (Variables|/Game/FPS/Blueprints/FPSArms_character.FPSArms_character_C|GetWood (Variables|Default|GetAs%20FPSArms%20Character)) (.wood _output_2))
          (bind _returnvalue (Game|SpawnActorfromClass (.actor _output_2) (Transformation|GetWorldTransform (Variables|/Script/Engine.Actor|GetRootComponent _ghostbuild)) "Undefined" "SelectDefaultAtRuntime" 0 0))
          (bind _asbuilding_base (Utilities|Casting|CastToBuildingBase (Variables|Default|GetHit%20Actor))
            (:then
              (bind _asbuilding_base_2 (Utilities|Casting|CastToBuildingBase _returnvalue))
              (Default|SetParentBuildandCollision _asbuilding_base_2 _asbuilding_base _hit_component)
              (Collision|SetCollisionEnabled _hit_component "NoCollision")
              (Utilities|Array|Add (Variables|/Game/FPS/Blueprints/Building/BuildingBase.BuildingBase_C|GetAvoidCollisionBoxes _asbuilding_base) _hit_component))
            (:CastFailed
              _))
          (Variables|/Game/FPS/Blueprints/FPSArms_character.FPSArms_character_C|SetWood _as_fpsarms_character (- (Variables|/Game/FPS/Blueprints/FPSArms_character.FPSArms_character_C|GetWood _as_fpsarms_character) (.wood _output_2)))
          (bind _result (Math|Integer|IncrementInt (Variables|/Game/FPS/Blueprints/GameMode/GM_EditMap.GM_EditMap_C|GetIndex _as_gm_edit_map))
            (:%20%20
              (Class|BPIBuilding|AddIndex(Message) _asbuilding_base _result)
              (Default|AddActor _as_gm_edit_map (Utilities|Struct|MakeStruct_MapSave _result (.actor _output) (.mesh _output) (Transformation|GetWorldTransform (Variables|/Script/Engine.Actor|GetRootComponent (Variables|Default|GetGhostBuild))) (.wood _output)))
              (Development|PrintString (Utilities|String|ToString(Integer) _result)))))))))

(fn DetectSnappingBox
  (bind _hit_actor (Variables|Default|GetHit%20Actor))
  (Utilities|Casting|CastToBuildingBase _hit_actor)
  (Utilities|IsValid _hit_actor
    (:Is%20Valid
      (Utilities|IsValid (Variables|Default|GetHit%20Component)
        (:Is%20Valid
          (Class|BPIBuilding|ReturnSnappingBox(Message) (Variables|Default|GetHit%20Actor) (.type (Utilities|Array|Get(acopy) (Variables|Default|GetBuildables) (Variables|Default|GetCurrentBuildId))))
          (return))))))

(fn EditBuild
  (Components|StaticMesh|SetStaticMesh (Variables|/Game/FPS/Blueprints/Building/BP_GhostBuild.BP_GhostBuild_C|GetStaticMesh (Variables|Default|GetGhostBuild)) (Utilities|Array|Get(acopy) (Utilities|Select :Index (Variables|Default|GetCurrentBuildId) :Option%200 (Variables|Default|GetFoundationTypes) :Option%201 (Variables|Default|GetFoundationTriangleTypes) :Option%202 (Variables|Default|GetWallTypes) :Option%203 (Variables|Default|GetFloorTypes) :Option%204 (Variables|Default|GetFloorTriangleTypes) :Option%205 (Variables|Default|GetRoofTypes)) (Variables|Default|GetEditId))))

(fn BuildGhostColor
  (bind _ghostbuild (Variables|Default|GetGhostBuild))
  (bind _staticmesh (Variables|/Game/FPS/Blueprints/Building/BP_GhostBuild.BP_GhostBuild_C|GetStaticMesh _ghostbuild))
  ;[1 1 1] for loop to iterate through all the materials on the ghost build mesh
  (for _index (range 0 (- (Rendering|Material|GetNumMaterials (Variables|/Game/FPS/Blueprints/Building/BP_GhostBuild.BP_GhostBuild_C|GetStaticMesh (Variables|Default|GetGhostBuild))) 1))
    (if (Variables|Default|GetCanBuild)
      (Rendering|Material|SetMaterial _staticmesh _index "/Game/FPS/Blueprints/Building/GhostGreen.GhostGreen")
      (else
        (Rendering|Material|SetMaterial _staticmesh _index "/Game/FPS/Blueprints/Building/GhostRed.GhostRed")))))

(fn BuildOnlyonSnapping
  (bind _ghostbuild (Variables|Default|GetGhostBuild))
  (bind _staticmesh (Variables|/Game/FPS/Blueprints/Building/BP_GhostBuild.BP_GhostBuild_C|GetStaticMesh _ghostbuild))
  (bind _staticmesh_2 (Variables|/Script/Engine.StaticMeshComponent|GetStaticMesh _staticmesh))
  (bind _returnvalue (== _staticmesh_2 "/Game/FPS/Blueprints/Building/FoundationTriangle.FoundationTriangle"))
  (bind _returnvalue_2 (== _staticmesh_2 "/Game/FPS/Blueprints/Building/Foundation.Foundation"))
  (bind _returnvalue_3 (or _returnvalue_2 _returnvalue))
  (bind _asbuilding_base (Utilities|Casting|CastToBuildingBase (Variables|Default|GetHit%20Actor))
    (:then
      (Variables|Default|SetHitFloor false)
      (if (== (Variables|Default|GetHit%20Component) (Variables|/Game/FPS/Blueprints/Building/BuildingBase.BuildingBase_C|GetStaticMesh _asbuilding_base))
        (Variables|Default|SetCanBuild false :!label _label)
        (else
          (Variables|Default|SetCanBuild true :!label _label_2))))
    (:CastFailed
      (Variables|Default|SetHitFloor true)
      (if _returnvalue_3
        (goto _label_2)
        (else
          (goto _label)))))
  (return (select (and _returnvalue_3 (Variables|Default|GetHitFloor)) (Variables|Default|GetSpawnTransform) (Transformation|GetWorldTransform (Variables|Default|GetHit%20Component)))))

(fn DisableAllSnappinginBuild
  (bind _last_hit_building (Variables|Default|GetLast%20Hit%20Building))
  (Utilities|IsValid _last_hit_building
    (:Is%20Valid
      (Default|DisableAllSnappingBoxes _last_hit_building))
    (:Is%20Not%20Valid
      _))
  (bind _asbuilding_base (Utilities|Casting|CastToBuildingBase (Variables|Default|GetHit%20Actor)))
  (Default|DisableAllSnappingBoxes _asbuilding_base))

(fn EnableAllSnappinginBuild
  (bind _last_hit_building (Variables|Default|GetLast%20Hit%20Building))
  (Utilities|IsValid _last_hit_building
    (:Is%20Valid
      (Default|EnableAllSnappingBoxes _last_hit_building))
    (:Is%20Not%20Valid
      _))
  (bind _asbuilding_base (Utilities|Casting|CastToBuildingBase (Variables|Default|GetHit%20Actor)))
  (Default|EnableAllSnappingBoxes _asbuilding_base))

(fn BuildOnlyonSnapping2
  (bind _ghostbuild (Variables|Default|GetGhostBuild))
  (bind _staticmesh (Variables|/Game/FPS/Blueprints/Building/BP_GhostBuild.BP_GhostBuild_C|GetStaticMesh _ghostbuild))
  (bind _staticmesh_2 (Variables|/Script/Engine.StaticMeshComponent|GetStaticMesh _staticmesh))
  (bind _returnvalue (== _staticmesh_2 "/Game/FPS/Blueprints/Building/FoundationTriangle.FoundationTriangle"))
  (bind _returnvalue_2 (== _staticmesh_2 "/Game/FPS/Blueprints/Building/Foundation.Foundation"))
  (bind _returnvalue_3 (or _returnvalue_2 _returnvalue))
  (bind _asbuilding_base (Utilities|Casting|CastToBuildingBase (Variables|Default|GetHit%20Actor))
    (:then
      (Variables|Default|SetHitFloor false)
      (if (== (Variables|Default|GetHit%20Component) (Variables|/Game/FPS/Blueprints/Building/BuildingBase.BuildingBase_C|GetStaticMesh _asbuilding_base))
        (Variables|Default|SetCanBuild false :!label _label)
        (else
          (Variables|Default|SetCanBuild true :!label _label_2))))
    (:CastFailed
      (Variables|Default|SetHitFloor true)
      (if _returnvalue_3
        (goto _label_2)
        (else
          (goto _label)))))
  (return (select (and _returnvalue_3 (Variables|Default|GetHitFloor)) (Variables|Default|GetSpawnTransform) (Variables|Default|GetSnapTransform))))

(fn EditBuilding
  (params (StaticMesh :type Static%20Mesh%20Object%20Reference)))

(fn ReturnSnappingBox
  (params (BuildType :type Integer))
  (return 0))

(fn ReturnSnappingBox2
  (params (BuildType :type Integer))
  (return false))