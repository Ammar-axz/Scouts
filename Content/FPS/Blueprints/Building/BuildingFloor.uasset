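; BuildingFloor is a floor piece for a building system that supplies snap points for attaching other build pieces.
; ReturnSnappingBox maps the build type to one of four box sets (wall, floor, triangle floor or roof), passes it to SetCollisions and returns it.
; Several build types share the wall or floor set.
; The EditBuilding event is empty, with its mesh-swap node left unconnected, and the construction script only calls the parent.
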(event EventBeginPlay
  (|CallParentFunction) ; This node is disabled and will not be called.\nDrag off pins to build functionality.
)

(event Collision|EventActorBeginOverlap
  (params (OtherActor :type Actor%20Object%20Reference))
  (|CallParentFunction OtherActor) ; This node is disabled and will not be called.\nDrag off pins to build functionality.
)

(event EventTick
  (params (DeltaSeconds :type Float%20%28single-precision%29))
  (|CallParentFunction DeltaSeconds) ; This node is disabled and will not be called.\nDrag off pins to build functionality.
)

(event EventEditBuilding
  (params (StaticMesh :type Static%20Mesh%20Object%20Reference)))

(fn ConstructionScript
  (|CallParentFunction))

(fn ReturnSnappingBox
  (params (BuildType :type Integer))
  (bind _wall2 (Variables|Default|GetWall2))
  (bind _wall3 (Variables|Default|GetWall3))
  (bind _wall4 (Variables|Default|GetWall4))
  (bind _floortri4 (Variables|Default|GetFloorTri4))
  (bind _floortri3 (Variables|Default|GetFloorTri3))
  (bind _floortri2 (Variables|Default|GetFloorTri2))
  (bind _floor1 (Variables|Default|GetFloor1))
  (bind _floor2 (Variables|Default|GetFloor2))
  (bind _floor3 (Variables|Default|GetFloor3))
  (bind _roof2 (Variables|Default|GetRoof2))
  (bind _roof3 (Variables|Default|GetRoof3))
  (bind _roof4 (Variables|Default|GetRoof4))
  (bind _roof1 (Variables|Default|GetRoof1))
  (bind _wall1 (Variables|Default|GetWall1))
  (bind _floor4 (Variables|Default|GetFloor4))
  (bind _floortri1 (Variables|Default|GetFloorTri1))
  (bind _array (Utilities|Array|MakeArray _floor1 _floor2 _floor3 _floor4))
  (bind _array_2 (Utilities|Array|MakeArray _wall1 _wall2 _wall3 _wall4))
  (bind _array_3 (Utilities|Array|MakeArray _roof2 _roof3 _roof4 _roof1))
  (bind _array_4 (Utilities|Array|MakeArray _floortri1 _floortri2 _floortri3 _floortri4))
  (switch int BuildType
    (:2
      _)
    (:3
      (CallFunction|SetCollisions _array :!label _label)
      (return _array))
    (:4
      (CallFunction|SetCollisions _array_4)
      (return _array_4))
    (:5
      (CallFunction|SetCollisions _array_3)
      (return _array_3))
    (:8
      _)
    (:9
      _)
    (:10
      _)
    (:11
      (goto _label))
    (:13
      _)
    (:14
      _))
  (CallFunction|SetCollisions _array_2)
  (return _array_2))