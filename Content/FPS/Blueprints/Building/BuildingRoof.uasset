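; Roof piece for a modular building system, derived from a parent building class and supplying the snap boxes for attaching other pieces.
; ReturnSnappingBox clears all boxes through the parent, then enables and returns those matching the requested build type, with several types sharing wall, floor or other sets.
; The EditBuilding event is empty, leaving its static mesh swap unconnected, and the construction script only calls the parent.
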(event EventBeginPlay
  (|CallParentFunction) ; This node is disabled and will not be called.\nDrag off pins to build functionality.
)

(event Collision|EventActorBeginOverlap
  (params (OtherActor :type Actor%20Object%20Reference))
  (|CallParentFunction OtherActor) ; This node is disabled and will not be called.\nDrag off pins to build functionality.
)

(event EventTick
  (params (DeltaSeconds :type Float%20%28single-precision%29))
  (|CallParentFunction DeltaSeconds) ; This node is disabled and will not be called.\nDrag off pins to build functionality.
)

(event EventEditBuilding
  (params (StaticMesh :type Static%20Mesh%20Object%20Reference)))

(fn ConstructionScript
  (|CallParentFunction))

(fn ReturnSnappingBox
  (params (BuildType :type Integer))
  (bind _array (Utilities|Array|MakeArray 0))
  (bind _array_2 (Utilities|Array|MakeArray 0 0))
  (bind _floor1 (Variables|Default|GetFloor1))
  (bind _wall (Variables|Default|GetWall))
  (bind _floor2 (Variables|Default|GetFloor2))
  (bind _array_3 (Utilities|Array|MakeArray _floor1 _floor2))
  (bind _array_4 (Utilities|Array|MakeArray _wall))
  (CallFunction|DisableAllSnappingBoxes)
  (switch int BuildType
    (:2
      _)
    (:3
      (CallFunction|SetCollisions _array_3 :!label _label)
      (return _array_3))
    (:4
      (CallFunction|SetCollisions _array_2 :!label _label_2)
      (return _array_2))
    (:5
      (CallFunction|SetCollisions _array)
      (return _array))
    (:8
      _)
    (:9
      _)
    (:10
      _)
    (:11
      (goto _label))
    (:12
      (goto _label_2)))
  (CallFunction|SetCollisions _array_4)
  (return _array_4))

(fn DisableAllSnappingBoxes
  (params (Array :type Array%20of%20Primitive%20Component%20Object%20References))
  (|CallParentFunction (Utilities|Array|MakeArray 0 0 (Variables|Default|GetFloor1) (Variables|Default|GetWall) (Variables|Default|GetFloor2) 0))
  (return))