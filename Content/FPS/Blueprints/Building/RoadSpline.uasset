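; RoadSpline is an actor that builds a road from spline mesh segments along a Spline component.
; AddSplinePoint appends world-space points to the spline.
; GenerateMesh divides the spline by ForwardAxisLength and adds a movable, collidable spline mesh per segment, using RoadStart first and RoadMesh after.
; Segment ends are sampled by distance in world space, except start tangents, which use local space; construction script and events are empty.
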(event Collision|EventActorBeginOverlap
  (params (OtherActor :type Actor%20Object%20Reference)))

(event EventTick
  (params (DeltaSeconds :type Float%20%28single-precision%29)))

(fn ConstructionScript)

(fn AddSplinePoint
  (params (Location :type Vector%20%28by%20ref%29))
  (Spline|AddSplinePoint (Variables|Default|GetSpline) Location "World" true))

(fn GenerateMesh
  (bind _spline (Variables|Default|GetSpline))
  (bind _forwardaxislength (Variables|Default|GetForwardAxisLength))
  (for _index (range 0 (- (/ (Spline|GetSplineLength (Variables|Default|GetSpline)) (Variables|Default|GetForwardAxisLength)) 1))
    (bind _returnvalue (AddComponent|AddSplineMeshComponent false))
    (Transformation|SetMobility _returnvalue "Movable")
    (if (== _index 0)
      (Components|StaticMesh|SetStaticMesh _returnvalue "/Game/FPS/Blueprints/Building/RoadStart.RoadStart")
      (else
        (Components|StaticMesh|SetStaticMesh _returnvalue "/Game/FPS/Blueprints/Building/RoadMesh.RoadMesh")))
    (SplineMesh|SetForwardAxis _returnvalue "X" true)
    (SplineMesh|SetStartandEnd _returnvalue (Spline|GetLocationatDistanceAlongSpline _spline (Math|Conversions|ToFloat(Integer) (* _index _forwardaxislength)) "World") (Spline|GetTangentatDistanceAlongSpline _spline (Math|Conversions|ToFloat(Integer) (* _index _forwardaxislength)) "Local") (Spline|GetLocationatDistanceAlongSpline _spline (Math|Conversions|ToFloat(Integer) (* (+ _index 1) _forwardaxislength)) "World") (Spline|GetTangentatDistanceAlongSpline _spline (Math|Conversions|ToFloat(Integer) (* (+ _index 1) _forwardaxislength)) "World") true :!class /Script/Engine.SplineMeshComponent)
    (Collision|SetCollisionEnabled _returnvalue "QueryAndPhysics")))