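; Chaos field actor that applies a bullet's destruction impulse to geometry collections around a sphere component.
; The BulletDamage event applies internal cluster strain from a linear radial falloff, multiplied by a subtract operator field built on FieldMagnitude.
; It then applies radial linear velocity from the sphere's center, culled by a similar subtract operator rather than the falloff.
; The actor destroys itself after a short delay.
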(event Custom|BulletDamage
  (bind _fieldsystemcomponent (Variables|Field|GetFieldSystemComponent))
  (bind _sphere (Variables|Default|GetSphere))
  (bind _returnresultsterminal (Variables|Default|GetReturnResultsTerminal))
  (bind _uniformscalar (Variables|Default|GetUniformScalar))
  (bind _field_magnitude (Variables|Default|GetField%20Magnitude))
  (bind _operatorfield (Variables|Default|GetOperatorField))
  (bind _returnvalue (Transformation|GetWorldLocation _sphere))
  (bind _returnvalue_2 (Class|ReturnResultsTerminal|SetReturnResultsTerminal _returnresultsterminal))
  (bind _returnvalue_3 (Class|UniformScalar|SetUniformScalar _uniformscalar _field_magnitude))
  (bind _returnvalue_4 (Field|SetOperatorField _operatorfield 1.0 _returnvalue_2 _returnvalue_3 "Field_Substract"))
  (Class|FieldSystemComponent|ApplyPhysicsField _fieldsystemcomponent true "Field_InternalClusterStrain" 0 (Field|SetOperatorField (Variables|Default|GetOperatorFieldFallOff) 1.0 (Field|SetRadialFalloff (Variables|Default|GetRadialFalloff) (Variables|Default|GetField%20Magnitude) 0.0 1e+01 0.0 (Components|Sphere|GetScaledSphereRadius _sphere) _returnvalue "Field_Falloff_Linear") _returnvalue_4 "Field_Multiply"))
  (Class|FieldSystemComponent|ApplyPhysicsField _fieldsystemcomponent true "Field_LinearVelocity" 0 (Field|SetCullingField (Variables|Default|GetCullingField) _returnvalue_4 (Field|SetRadialVector (Variables|Default|GetRadialVector) 1.0 _returnvalue) "Field_Culling_Outside"))
  (Utilities|FlowControl|Delay 0.2)
  (Actor|DestroyActor))

(event EventBeginPlay)

(fn ConstructionScript)