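; FPS game mode Blueprint that provides a player spawn routine.
; SpawnPlayer destroys the controller's current pawn, spawns an FPSArms_character at PlayerStartLocation, and possesses it.
; PlayerStartLocation gathers PlayerStart actors, but its loop and "Taken" tagging are disconnected, so the returned element is never selected.
; A countdown timer widget and restart-at-zero logic also sit unconnected, leaving BeginPlay and Tick empty.
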(event EventBeginPlay
  ;[1 1 1] TIMER
)

(event EventTick
  (params (DeltaSeconds :type Float%20%28single-precision%29))
  ;[1 1 1] TIMER
)

(fn ConstructionScript)

(fn PlayerStartLocation
  (bind _outactors (Actor|GetAllActorsOfClass "/Script/Engine.PlayerStart"))
  (return (Transformation|GetActorLocation (stale _array_element))))

(fn SpawnPlayer
  (params (PlayerController :type Player%20Controller%20Object%20Reference))
  (bind _returnvalue (Pawn|GetControlledPawn PlayerController))
  (Utilities|IsValid _returnvalue
    (:Is%20Valid
      (Actor|DestroyActor _returnvalue))
    (:Is%20Not%20Valid
      _))
  (bind _returnvalue_2 (Game|SpawnActorfromClass "/Game/FPS/Blueprints/FPSArms_character.FPSArms_character_C" (Math|Transform|MakeTransform (CallFunction|PlayerStartLocation) "0, 0, 0" "1.000000,1.000000,1.000000") "AlwaysSpawn" "MultiplyWithRoot" 0 0))
  (Pawn|Possess PlayerController _returnvalue_2))