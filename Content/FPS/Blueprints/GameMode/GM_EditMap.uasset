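; Game mode for map editing that persists spawned actors in a BP_MapSave, using the slot name from Game_Instance_1.
; BeginPlay creates the save or respawns its stored actors, passing each its index and deducting their summed Wood from the player character.
; AddActor and DeleteActor update the index-keyed actor map and save immediately; the current Index is set from the last loaded entry.
; An unconnected chain would give the player a BuildingPlan inventory item.
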(event Custom|DeleteActor
  (params (Index :type Integer))
  (bind _savegameslot (Variables|Default|GetSaveGameSlot))
  (bind _as_bp_map_save (Variables|Default|GetAs%20BP%20Map%20Save))
  (Utilities|Map|Remove (Variables|/Game/FPS/Blueprints/BP_MapSave.BP_MapSave_C|GetActorsToSpawn _as_bp_map_save) Index)
  (SaveGame|SaveGametoSlot _as_bp_map_save _savegameslot)
  (Development|PrintString _savegameslot))

(event Custom|AddActor
  (params (ActorData :type Struct%20Map%20Save%20Structure))
  (bind _savegameslot (Variables|Default|GetSaveGameSlot))
  (bind _as_bp_map_save (Variables|Default|GetAs%20BP%20Map%20Save))
  (Utilities|Map|Add (Variables|/Game/FPS/Blueprints/BP_MapSave.BP_MapSave_C|GetActorsToSpawn _as_bp_map_save) (Variables|Default|GetIndex) ActorData)
  (SaveGame|SaveGametoSlot _as_bp_map_save _savegameslot)
  (Development|PrintString _savegameslot))

(event EventTick
  (params (DeltaSeconds :type Float%20%28single-precision%29)))

(event EventBeginPlay
  (bind _asgame_instance_1 (Utilities|Casting|CastToGame_Instance_1 (Game|GetGameInstance)))
  (Development|PrintString (Variables|/Game/FPS/Blueprints/GameMode/Game_Instance_1.Game_Instance_1_C|GetSaveSlotName _asgame_instance_1))
  (Variables|Default|SetSaveGameSlot (Variables|/Game/FPS/Blueprints/GameMode/Game_Instance_1.Game_Instance_1_C|GetSaveSlotName _asgame_instance_1))
  (bind _returnvalue (SaveGame|DoesSaveGameExist (Variables|Default|GetSaveGameSlot)))
  (if _returnvalue
    (bind _returnvalue_2 (SaveGame|LoadGamefromSlot (Variables|Default|GetSaveGameSlot)))
    (bind _asbp_map_save (Utilities|Casting|CastToBP_MapSave _returnvalue_2))
    (bind _output_get (Variables|Default|SetAs%20BP%20Map%20Save _asbp_map_save))
    (bind _values (Utilities|Map|Values (Variables|/Game/FPS/Blueprints/BP_MapSave.BP_MapSave_C|GetActorsToSpawn _output_get)))
    (for _array_element _values
      (bind _returnvalue_3 (Game|SpawnActorfromClass (.actor _array_element) (.transform _array_element) "Undefined" "MultiplyWithRoot" 0 0))
      (Class|BPIBuilding|AddIndex(Message) _returnvalue_3 (.index _array_element))
      (Variables|Default|SetWood (+ (.wood _array_element) (Variables|Default|GetWood))))
    (bind _output_get_2 (Variables|Default|SetIndex (.index _array_element)))
    (Development|PrintString (Utilities|String|ToString(Integer) _output_get_2))
    (bind _asfpsarms_character (Utilities|Casting|CastToFPSArms_character (Game|GetPlayerCharacter 0)))
    (Variables|/Game/FPS/Blueprints/FPSArms_character.FPSArms_character_C|SetWood _asfpsarms_character (- (Variables|/Game/FPS/Blueprints/FPSArms_character.FPSArms_character_C|GetWood _asfpsarms_character) (Variables|Default|GetWood)))
    (Development|PrintString (Utilities|String|ToString(Integer) (Variables|Default|GetWood)))
    (else
      (bind _returnvalue_4 (SaveGame|CreateSaveGameObject "/Game/FPS/Blueprints/BP_MapSave.BP_MapSave_C"))
      (bind _output_get_3 (Variables|Default|SetAs%20BP%20Map%20Save _returnvalue_4))
      (SaveGame|SaveGametoSlot _output_get_3 (Variables|Default|GetSaveGameSlot)))))

(fn ConstructionScript)