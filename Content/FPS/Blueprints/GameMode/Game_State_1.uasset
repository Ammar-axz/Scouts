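; FPS game state that runs the match countdown and provides a helper for dropping items into the world.
; A timeline started on BeginPlay drives the seconds value, replaying as each minute is decremented and calling RestartGame on GAME_MODE_1 when time runs out.
; SpawnItemFromActor spawns an item's class in front of an actor, optionally ground-clamped by a downward trace, with query-only sphere collision.
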(event Custom|TimerOnSv
  (bind _seconds (Timeline|TimerTimeline PlayFromStart)
    (:Update
      (if (== _seconds 0.0)
        (if (== (Variables|Default|GetGameTimeMin) 0.0)
          (Class|GameMode|RestartGame (.AsGAME%20MODE%201 (Utilities|Casting|CastToGAME_MODE_1 (Game|GetGameMode))))
          (else
            (bind _result (Math|Float|DecrementFloat (Variables|Default|GetGameTimeMin))
              (:%20%20
                (Variables|Default|SetGameTimeMin _result)
                (Timeline|TimerTimeline PlayFromStart)))))
        (else
          (Variables|Default|SetGameTimeSec _seconds))))))

(event EventBeginPlay
  (CallFunction|TimeronSv))

(event EventTick
  (params (DeltaSeconds :type Float%20%28single-precision%29)))

(fn ConstructionScript)

(fn SpawnItemfromActor
  (params (ItemObject :type Item%20Object%20Object%20Reference) (Actor :type Actor%20Object%20Reference) (GroundClamp :type Boolean))
  (Utilities|FlowControl|Sequence
    (:then_0
      (LocalVariables|SetSpawnLocation%28Local%29 (+ (Transformation|GetActorLocation Actor) (* (Transformation|GetActorForwardVector Actor) (Variables|Default|GetSpawnForwardVector))))
      (if GroundClamp
        (bind (_outhit _returnvalue) (Collision|LineTraceByChannel (LocalVariables|GetSpawnLocation%28Local%29) (- (LocalVariables|GetSpawnLocation%28Local%29) "0.000000,0.000000,1000.000000") "TraceTypeQuery1" false 0 "None"))
        (if _returnvalue
          (LocalVariables|SetSpawnLocation%28Local%29 (.Location (Collision|BreakHitResult _outhit))))))
    (:then_1
      (bind _returnvalue_2 (Game|SpawnActorfromClass (Default|GetItemClass ItemObject) (Math|Transform|MakeTransform (LocalVariables|GetSpawnLocation%28Local%29) "0, 0, 0" "1.000000,1.000000,1.000000") "Undefined" 0 0))
      (Collision|SetCollisionEnabled (Variables|/Game/FPS/Blueprints/Inventory/Items/ItemPickupBPs/Item_Base.Item_Base_C|GetSphere _returnvalue_2) "QueryOnly"))))