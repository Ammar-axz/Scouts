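; Player controller for the FPS mode that requests the player's spawn and sets up the local HUD and input.
; On BeginPlay, only for the local controller, it calls OnSv, which casts the game mode to GAME_MODE_1 and calls SpawnPlayer with itself.
; If the game state is a valid Game_State_1, it then adds the timer, crosshair and game HUD widgets and the default Enhanced Input mapping context.
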(event Custom|OnSv
  (bind _asgame_mode_1 (Utilities|Casting|CastToGAME_MODE_1 (Game|GetGameMode)))
  (Default|SpawnPlayer _asgame_mode_1 self))

(event EventBeginPlay
  (if (Pawn|IsLocalPlayerController)
    (CallFunction|OnSv)
    (Utilities|IsValid (.AsGame%20State%201 (Utilities|Casting|CastToGame_State_1 (Game|GetGameState)))
      (:Is%20Valid
        (bind _returnvalue (UserInterface|CreateWidget "/Game/FPS/Blueprints/UI/TImer_ui.TImer_ui_C"))
        (UserInterface|Viewport|AddtoViewport _returnvalue 0)
        (bind _returnvalue_2 (UserInterface|CreateWidget "/Game/FPS/Blueprints/UI/Crosshair.Crosshair_C"))
        (bind _returnvalue_3 (UserInterface|CreateWidget "/Game/FPS/Blueprints/UI/Game_Hud.Game_Hud_C"))
        (UserInterface|Viewport|AddtoViewport _returnvalue_2 0)
        (Input|AddMappingContext (PlayerController|LocalPlayerSubsystems|GetEnhancedInputLocalPlayerSubsystem) "/Game/VehicleTemplate/Input/IMC_Default.IMC_Default" 0 "(bIgnoreAllPressedKeysUntilRelease=True,bForceImmediately=False)") ; Adding the Input Mapping Context needed to trigger the proper Input Actions.
      ))))

(fn ConstructionScript)