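; GridComponent builds a Rows by Columns grid of GridCell actors over a static mesh, tagged with the "Building" build type.
; Cell size comes from dividing the mesh's world scale by the row and column counts, shrunk slightly to show gaps.
; The first cell snaps to the mesh and anchors the offsets of the others; cells are stored in nested 2D arrays.
; CheckAdjacentCells is a stub that only loops over that array.
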(fn CalculateGridBoxes
  (params (StaticMesh :type Scene%20Component%20Object%20Reference))
  (bind _returnvalue (Transformation|GetWorldScale StaticMesh))
  (Variables|Default|SetRowWidth (/ (.x _returnvalue) (Math|Conversions|ToFloat(Integer) (Variables|Default|GetRows))))
  (bind _output_get (Variables|Default|SetColumnWidth (/ (.y _returnvalue) (Math|Conversions|ToFloat(Integer) (Variables|Default|GetColumns)))))
  (Development|PrintString (Utilities|String|ToString(Float) _output_get)))

(fn SpawnGridBoxes
  (params (StaticMesh :type Scene%20Component%20Object%20Reference) (BuildablePlane :type Actor%20Object%20Reference) (BuildType :type String) (grid%20Z :type Float%20%28double-precision%29))
  (bind _returnvalue (Transformation|GetRelativeTransform StaticMesh))
  (CallFunction|CalculateGridBoxes StaticMesh)
  (for _index (range 1 (Variables|Default|GetRows))
    (Utilities|Array|Clear (Variables|Default|GetGridCellX))
    (if (== _index 1)
      _
      (else
        (Variables|Default|SetGridLocation (Math|Vector|MakeVector (+ (* (Variables|Default|GetRowWidth) 1e+02) (.x (Variables|Default|GetGridLocation))) (.y (LocalVariables|GetlocY)) (.z (Variables|Default|GetGridLocation))))))
    (for _index_2 (range 1 (Variables|Default|GetColumns))
      (if (== _index_2 1)
        _
        (else
          (bind _output_get (Variables|Default|SetGridLocation (Math|Vector|MakeVector (.x (Variables|Default|GetGridLocation)) (+ (* (Variables|Default|GetColumnWidth) 1e+02) (.y (Variables|Default|GetGridLocation))) (.z (Variables|Default|GetGridLocation)))))))
      (bind _returnvalue_2 (Game|SpawnActorfromClass "/Game/FPS/Blueprints/Grid/GridCell.GridCell_C" (Math|Transform|MakeTransform _output_get (.rotation (Math|Transform|MakeTransform _output_get (.rotation _returnvalue) (.scale _returnvalue))) "1.000000,1.000000,1.000000") "AlwaysSpawn" 0 0))
      (if (== _index 1)
        (if (== _index_2 1)
          (Transformation|AttachComponentToComponent _returnvalue_2 StaticMesh "None" "SnapToTarget" "SnapToTarget" "SnapToTarget" true)
          (bind _output_get_2 (Variables|Default|SetGridLocation (Transformation|GetWorldLocation (Variables|/Script/Engine.Actor|GetRootComponent _returnvalue_2))))
          (LocalVariables|SetlocY _output_get_2)
          (else
            (Transformation|AttachComponentToComponent _returnvalue_2 StaticMesh "None" "KeepWorld" "SnapToTarget" "SnapToTarget" true :!label _label)))
        (else
          (goto _label)))
      (Variables|/Game/FPS/Blueprints/Grid/GridCell.GridCell_C|SetBuildType _returnvalue_2 "Building")
      (Transformation|SetWorldScale3D (Variables|/Script/Engine.Actor|GetRootComponent _returnvalue_2) (Math|Vector|MakeVector (- (Variables|Default|GetRowWidth) 0.1) (- (Variables|Default|GetColumnWidth) 0.1) grid%20Z))
      (Variables|/Game/FPS/Blueprints/Grid/GridCell.GridCell_C|SetGridX _returnvalue_2 _index)
      (Variables|/Game/FPS/Blueprints/Grid/GridCell.GridCell_C|SetGridY _returnvalue_2 _index_2)
      (Variables|/Game/FPS/Blueprints/Grid/GridCell.GridCell_C|SetGridComponent _returnvalue_2 self)
      (Utilities|Array|SetArrayElem (Variables|Default|GetGridCellX) _index_2 _returnvalue_2 true))
    (Utilities|Array|SetArrayElem (Variables|Default|GetGridCellY) _index (Utilities|Struct|MakeGridCell2DArray (Variables|Default|GetGridCellX)) true)))

(fn CheckAdjacentCells
  (for _array_element (Variables|Default|GetGridCellY)
    (for _array_element_2 (.gridcellx _array_element)
      _)))