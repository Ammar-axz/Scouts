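; Grid-based inventory component that stores multi-tile items in a flat Columns × Rows array, with every covered cell referencing its item.
; TryAddItem scans for the first spot where the item's footprint fits, retrying once rotated, using tile/index conversion and bounds-check helpers.
; GetAllItems collapses cells into a map of unique items to top-left tiles.
; Adds and removals set a dirty flag, so Tick broadcasts OnInventoryChanged at most once per frame.
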(event EventTick
  (params (DeltaSeconds :type Float%20%28single-precision%29))
  (if (Variables|Default|GetisDirty)
    (Variables|Default|SetisDirty false)
    (Default|CallOnInventoryChanged)))

(event EventBeginPlay
  (Utilities|Array|Resize (Variables|Default|GetItems) (* (Variables|Default|GetColumns) (Variables|Default|GetRows))))

(fn TryAddItem
  (params (ItemObject :type Item%20Object%20Object%20Reference))
  (Utilities|IsValid ItemObject
    (:Is%20Valid
      (for (_ _array_index) (Variables|Default|GetItems) :!label _label
        (bind _result (CallFunction|IsRoomAvailable ItemObject _array_index))
        (if _result
          (CallFunction|AddItemat ItemObject _array_index)
          (return true)))
      (Utilities|FlowControl|Sequence
        (:then_0
          (Utilities|FlowControl|DoOnce false
            (:Completed
              (Default|Rotate ItemObject)
              (goto _label))))
        (:then_1
          (Default|Rotate ItemObject)
          (return false))))))

(fn IsRoomAvailable
  (params (ItemObject :type Item%20Object%20Object%20Reference) (TopLeftIndex :type Integer))
  (Utilities|FlowControl|Sequence
    (:then_0
      (bind _tile (Utilities|ForEachIndex ItemObject TopLeftIndex)
        (:LoopBody
          (Utilities|IsTileValid _tile
            (:true
              (bind (_valid _itemobject) (CallFunction|GetItematIndex (CallFunction|TiletoIndex _tile)))
              (if _valid
                (Utilities|IsValid _itemobject
                  (:Is%20Valid
                    (return false)))
                (else
                  (return false))))
            (:false
              (return false))))))
    (:then_1
      (return true))))

(fn IndextoTile
  (params (Index :type Integer))
  (bind _columns (Variables|Default|GetColumns))
  (return (Utilities|Struct|MakeTiles (Math|Integer|%(Integer) Index _columns) (/ Index _columns))))

(fn GetItematIndex
  (params (index :type Integer))
  (bind _items (Variables|Default|GetItems))
  (if (Utilities|Array|IsValidIndex _items index)
    (return true (Utilities|Array|Get(acopy) _items index))
    (else
      (return false 0))))

(fn TiletoIndex
  (params (Tile :type Tiles%20Structure))
  (return (+ (.x Tile) (* (.y Tile) (Variables|Default|GetColumns)))))

(fn AddItemat
  (params (ItemObject :type Item%20Object%20Object%20Reference) (TopLeftIndex :type Integer))
  (bind _tile (Utilities|ForEachIndex ItemObject TopLeftIndex)
    (:LoopBody
      (Utilities|Array|SetArrayElem (Variables|Default|GetItems) (CallFunction|TiletoIndex _tile) ItemObject))
    (:Completed
      (Variables|Default|SetisDirty true))))

(fn GetAllItems
  (for (_array_element _array_index) (Variables|Default|GetItems)
    (bind _output_get (LocalVariables|SetCurrentItemObject%28Local%29 _array_element))
    (Utilities|IsValid _output_get
      (:Is%20Valid
        (if (not (Utilities|Map|Contains (LocalVariables|GetAllItems%28Local%29) _array_element))
          (Utilities|Map|Add (LocalVariables|GetAllItems%28Local%29) (LocalVariables|GetCurrentItemObject%28Local%29) (CallFunction|IndextoTile _array_index))))))
  (return (LocalVariables|GetAllItems%28Local%29)))

(fn RemoveItem
  (params (ItemObject :type Item%20Object%20Object%20Reference))
  (Utilities|IsValid ItemObject
    (:Is%20Valid
      (for (_array_element _array_index) (Variables|Default|GetItems)
        (if (== _array_element ItemObject)
          (Utilities|Array|SetArrayElem (Variables|Default|GetItems) _array_index 0)
          (Variables|Default|SetisDirty true))))))