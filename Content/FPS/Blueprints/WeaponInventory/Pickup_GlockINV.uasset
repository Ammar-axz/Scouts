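; Glock pickup Blueprint for the FPS weapon inventory, a child class that supplies Glock-specific data to its parent.
; The construction script runs the parent's, then sets the weapon name, class to set and secondary-weapon struct, which references this pickup class.
; The sphere overlap event is empty; leftover nodes for filling the character's inventory or secondary slot and destroying the pickup are disconnected and never run.
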(event OnComponentBeginOverlap(Sphere)
  (params (OverlappedComponent :type Primitive%20Component%20Object%20Reference) (OtherActor :type Actor%20Object%20Reference) (OtherComp :type Primitive%20Component%20Object%20Reference) (OtherBodyIndex :type Integer) (bFromSweep :type Boolean) (SweepResult :type Hit%20Result%20Structure%20%28by%20ref%29)))

(fn ConstructionScript
  (|CallParentFunction)
  (Variables|Default|SetWeaponEquipped "GLOCK")
  (Variables|Default|SetClassToSet "/Game/FPS/Blueprints/Weapons/Weapon_Glock.Weapon_Glock_C")
  (Variables|Default|SetPickSec (Utilities|Struct|MakeWeaponsDetails "NewEnumerator1" "/Game/FPS/Blueprints/Weapons/Weapon_Glock.Weapon_Glock_C" 20 20 0.0 0.0 0.0 0.05 false "Pickup_GlockINV_C" "NewEnumerator1" 0 0 "(bIsDynamicallyLoaded=False,DrawAs=Image,Tiling=NoTile,Mirroring=NoMirror,ImageType=NoImage,ImageSize=(X=32.000000,Y=32.000000),Margin=(Left=0.000000,Top=0.000000,Right=0.000000,Bottom=0.000000),TintColor=(SpecifiedColor=(R=1.000000,G=1.000000,B=1.000000,A=1.000000),ColorUseRule=UseColor_Specified),OutlineSettings=(CornerRadii=(X=0.000000,Y=0.000000,Z=0.000000,W=1.000000),Color=(SpecifiedColor=(R=0.000000,G=0.000000,B=0.000000,A=0.000000),ColorUseRule=UseColor_Specified),Width=0.000000,RoundingType=HalfHeightRadius,bUseBrushTransparency=False),ResourceObject=None,ResourceName=\"\",UVRegion=(Min=(X=0.000000,Y=0.000000),Max=(X=0.000000,Y=0.000000),bIsValid=False))" 0 0 0 "(X=0,Y=0)")))