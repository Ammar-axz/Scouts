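; Knife pickup Blueprint for the FPS weapon inventory, configured as a child of a parent pickup class.
; Its construction script runs the parent's, then sets the equipped weapon name and spawn class to the knife.
; The sphere overlap event is empty.
; Disconnected leftover nodes would add the weapon to the character's inventory, destroy the pickup, or spawn and attach it to the arms' primary gun socket.
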(event OnComponentBeginOverlap(Sphere)
  (params (OverlappedComponent :type Primitive%20Component%20Object%20Reference) (OtherActor :type Actor%20Object%20Reference) (OtherComp :type Primitive%20Component%20Object%20Reference) (OtherBodyIndex :type Integer) (bFromSweep :type Boolean) (SweepResult :type Hit%20Result%20Structure%20%28by%20ref%29)))

(fn ConstructionScript
  (|CallParentFunction)
  (Variables|Default|SetWeaponEquipped "KNIFE")
  (Variables|Default|SetClassToSet "/Game/FPS/Blueprints/Weapons/Knife.Knife_C"))