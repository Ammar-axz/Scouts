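; Secondary weapon pickup actor for the FPS weapon inventory.
; On BeginPlay it chains SetOnSv into SetMulti, which stores the pickup in player 0's FPSArms_character PickSec reference.
; The sphere overlap event is empty.
; Disconnected leftover logic would fill inventory slot 2, destroy the pickup and set Secondary to a hardcoded Glock, but it never runs.
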(event OnComponentBeginOverlap(Sphere)
  (params (OverlappedComponent :type Primitive%20Component%20Object%20Reference) (OtherActor :type Actor%20Object%20Reference) (OtherComp :type Primitive%20Component%20Object%20Reference) (OtherBodyIndex :type Integer) (bFromSweep :type Boolean) (SweepResult :type Hit%20Result%20Structure%20%28by%20ref%29)))

(event Custom|SetMulti
  (bind _asfpsarms_character (Utilities|Casting|CastToFPSArms_character (Game|GetPlayerCharacter 0)))
  (Variables|/Game/FPS/Blueprints/FPSArms_character.FPSArms_character_C|SetPickSec _asfpsarms_character self))

(event Custom|SetOnSv
  (CallFunction|SetMulti))

(event EventBeginPlay
  (CallFunction|SetonSv))

(fn ConstructionScript
  (|CallParentFunction))