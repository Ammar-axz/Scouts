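; USP pistol pickup for the weapon inventory, built as a child of a parent pickup Blueprint.
; Its construction script runs the parent's, then sets the weapon name, the class to set and a secondary-weapon struct referencing the USP weapon and this pickup.
; The sphere overlap event is empty; older logic for writing to the FPSArms_character inventory or Secondary slot is left disconnected.
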(event OnComponentBeginOverlap(Sphere)
  (params (OverlappedComponent :type Primitive%20Component%20Object%20Reference) (OtherActor :type Actor%20Object%20Reference) (OtherComp :type Primitive%20Component%20Object%20Reference) (OtherBodyIndex :type Integer) (bFromSweep :type Boolean) (SweepResult :type Hit%20Result%20Structure%20%28by%20ref%29)))

(fn ConstructionScript
  (|CallParentFunction)
  (Variables|Default|SetWeaponEquipped "USP")
  (Variables|Default|SetClassToSet "/Game/FPS/Blueprints/Weapons/Weapon_USP.Weapon_USP_C")
  (Variables|Default|SetPickSec (Utilities|Struct|MakeWeaponsDetails "NewEnumerator4" "/Game/FPS/Blueprints/Weapons/Weapon_USP.Weapon_USP_C" 12 12 0.0 0.0 0.0 0.0 false "Pickup_USPINV_C" "NewEnumerator1" 0 0 "(TintColor=(SpecifiedColor=(R=1.000000,G=1.000000,B=1.000000,A=1.000000),ColorUseRule=UseColor_Specified),DrawAs=Image,Tiling=NoTile,Mirroring=NoMirror,ImageType=NoImage,ImageSize=(X=32.000000,Y=32.000000),Margin=(Left=0.000000,Top=0.000000,Right=0.000000,Bottom=0.000000),ResourceObject=None,OutlineSettings=(CornerRadii=(X=0.000000,Y=0.000000,Z=0.000000,W=1.000000),Color=(SpecifiedColor=(R=0.000000,G=0.000000,B=0.000000,A=0.000000),ColorUseRule=UseColor_Specified),Width=0.000000,RoundingType=HalfHeightRadius,bUseBrushTransparency=False),UVRegion=(Min=(X=0.000000,Y=0.000000),Max=(X=0.000000,Y=0.000000),bIsValid=False),bIsDynamicallyLoaded=False,ResourceName=\"\")" 0 0 0 "(X=0,Y=0)")))