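; Base Blueprint for primary-slot FPS weapons, extending a parent weapon class.
; UnEquip saves the weapon's ammo, stats, pickup class and montages into the arms character's Primary struct.
; AmmoCheck and Shoot overrides skip while player 0 is reloading, otherwise play the weapon animation and call the parent; only AmmoCheck adds the gunshot sound.
; The Sphere overlap event does nothing, leaving a disconnected character cast.
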(event OnComponentBeginOverlap(Sphere)
  (params (OverlappedComponent :type Primitive%20Component%20Object%20Reference) (OtherActor :type Actor%20Object%20Reference) (OtherComp :type Primitive%20Component%20Object%20Reference) (OtherBodyIndex :type Integer) (bFromSweep :type Boolean) (SweepResult :type Hit%20Result%20Structure%20%28by%20ref%29)))

(event EventUnEquip
  (params (FPSArmsCharacter :type FPS%20Arms%20Character%20Object%20Reference))
  (Variables|/Game/FPS/Blueprints/FPSArms_character.FPSArms_character_C|SetPrimary FPSArmsCharacter (Utilities|Struct|MakeWeaponsDetails (Variables|Default|GetWeaponName) (Variables|Default|GetWeaponClass) (Variables|Default|GetAmmoCount) (Variables|Default|GetMaxAmmo) (Variables|Default|GetReloadTime) 0.0 (Variables|Default|GetBulletSpread) (Variables|Default|GetFireRate) (Variables|Default|GetAutoFire) (Variables|Default|GetPickupClass) (Variables|Default|GetType) (Variables|Default|GetAimDS_Anim_Montage) (Variables|Default|GetArms_Reload_Anim_Montage) "(TintColor=(SpecifiedColor=(R=1.000000,G=1.000000,B=1.000000,A=1.000000),ColorUseRule=UseColor_Specified),DrawAs=Image,Tiling=NoTile,Mirroring=NoMirror,ImageType=NoImage,ImageSize=(X=32.000000,Y=32.000000),Margin=(Left=0.000000,Top=0.000000,Right=0.000000,Bottom=0.000000),ResourceObject=None,OutlineSettings=(CornerRadii=(X=0.000000,Y=0.000000,Z=0.000000,W=1.000000),Color=(SpecifiedColor=(R=0.000000,G=0.000000,B=0.000000,A=0.000000),ColorUseRule=UseColor_Specified),Width=0.000000,RoundingType=HalfHeightRadius,bUseBrushTransparency=False),UVRegion=(Min=(X=0.000000,Y=0.000000),Max=(X=0.000000,Y=0.000000),bIsValid=False),bIsDynamicallyLoaded=False,ResourceName=\"\")" 0 0 0 "(X=0,Y=0)")))

(fn ConstructionScript
  (|CallParentFunction))

(fn AmmoCheck
  (if (not (Variables|/Game/FPS/Blueprints/FPSArms_character.FPSArms_character_C|GetIsReloading (.AsFPSArms%20Character (Utilities|Casting|CastToFPSArms_character (Game|GetPlayerCharacter 0)))))
    (Components|Animation|PlayAnimation (Variables|Default|GetWeapon) 0 false)
    (Audio|PlaySoundatLocation "/Game/FPS/FPS_PAWN/Gunshot.Gunshot" (Transformation|GetWorldLocation (Variables|Default|GetWeapon)) "0, 0, 0" 1.0 1.0 0.0 0 0 0 0)
    (|CallParentFunction)))

(fn Shoot
  (params (PlayerController :type Player%20Controller%20Object%20Reference) (PlayeCharacter :type FPS%20Arms%20Character%20Object%20Reference))
  (if (not (Variables|/Game/FPS/Blueprints/FPSArms_character.FPSArms_character_C|GetIsReloading (.AsFPSArms%20Character (Utilities|Casting|CastToFPSArms_character (Game|GetPlayerCharacter 0)))))
    (Components|Animation|PlayAnimation (Variables|Default|GetWeapon) 0 false)
    (|CallParentFunction 0 0)))