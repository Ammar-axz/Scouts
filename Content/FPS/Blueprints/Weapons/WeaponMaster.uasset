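; Base FPS weapon that loads its stats and montages from a data table row in the construction script.
; Fire loops automatic shots through a gate and retriggerable delay, while a timeline drives bullet spread.
; Shoot line-traces from the character's SprayPoint, subtracts health with headshot bonus, ragdolls at zero, and spawns tracer, decal and Chaos field on non-character or lethal hits.
; Reload plays weapon and arms montages, then refills ammo.
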(event Custom|Reload
  (params (Reload_Anim :type Anim%20Montage%20Object%20Reference) (FPS_ARms%20Ref :type FPS%20Arms%20Character%20Object%20Reference))
  (bind _output_get (Variables|Default|SetCharacter FPS_ARms%20Ref))
  (Variables|/Game/FPS/Blueprints/FPSArms_character.FPSArms_character_C|SetAttachLeft%20Hand%20to%20Weapon _output_get false)
  (Utilities|FlowControl|DoOnce false :!label _label
    (:Completed
      (Utilities|IsValid (Variables|/Script/Engine.ChildActorComponent|GetChildActor (Variables|/Game/FPS/Blueprints/FPSArms_character.FPSArms_character_C|GetWeaponChildActor (Variables|Default|GetCharacter)))
        (:Is%20Valid
          (if (< (Variables|Default|GetAmmoCount) (Variables|Default|GetMaxAmmo))
            (Variables|/Game/FPS/Blueprints/FPSArms_character.FPSArms_character_C|SetIsReloading (Variables|Default|GetCharacter) true)
            (Utilities|IsValid Reload_Anim
              (:Is%20Valid
                (Animation|Montage|PlayMontage (Variables|Default|GetWeapon) (Variables|Default|GetReload_Anim_Montage) 1.0 0.0 "Default"
                  (:then
                    (Animation|Montage|PlayMontage (Variables|/Game/FPS/Blueprints/FPSArms_character.FPSArms_character_C|GetFPSArms (Variables|Default|GetCharacter)) Reload_Anim 1.0 0.0 "Default"
                      (:OnCompleted
                        _)))))
              (:Is%20Not%20Valid
                _))
            (Variables|Default|SetAmmoCount (Variables|Default|GetMaxAmmo))
            (Variables|/Game/FPS/Blueprints/FPSArms_character.FPSArms_character_C|SetIsReloading (Variables|Default|GetCharacter) false)
            (Variables|/Game/FPS/Blueprints/FPSArms_character.FPSArms_character_C|SetAttachLeft%20Hand%20to%20Weapon (Variables|Default|GetCharacter) true)
            (goto _label Reset)))))))

(event Custom|Fire
  (params (Character :type FPS%20Arms%20Character%20Object%20Reference) (PlayerController :type Player%20Controller%20Object%20Reference))
  (Variables|Default|SetCharacter Character)
  (Utilities|IsValid (Variables|/Script/Engine.ChildActorComponent|GetChildActor (Variables|/Game/FPS/Blueprints/FPSArms_character.FPSArms_character_C|GetWeaponChildActor (Variables|Default|GetCharacter)))
    (:Is%20Valid
      (Utilities|FlowControl|Sequence
        (:then_0
          (if (> (Variables|Default|GetAmmoCount) 0)
            (if (Variables|Default|GetAutoFire)
              (Utilities|FlowControl|Sequence
                (:then_0
                  (goto _label Open))
                (:then_1
                  (Utilities|FlowControl|Gate true :!label _label
                    (:Exit
                      (Utilities|FlowControl|Sequence
                        (:then_0
                          (if true :!label _label_2
                            (CallFunction|AmmoCheck)
                            (CallFunction|Shoot PlayerController (Variables|Default|GetCharacter))
                            (Camera|PlayWorldCameraShake "/Game/FPS/Blueprints/WEaponCameraShake.WEaponCameraShake_C" (Transformation|GetActorLocation) 0.0 1e+02)
                            (CallFunction|SprayStart)
                            (Variables|/Game/FPS/Blueprints/FPSArms_character.FPSArms_character_C|SetLastShotTime (Variables|Default|GetCharacter) (Utilities|Time|GetGameTimeinSeconds))
                            (Variables|/Game/FPS/Blueprints/FPSArms_character.FPSArms_character_C|SetUseTimeSinceLastShot (Variables|Default|GetCharacter) true)))
                        (:then_1
                          (Utilities|FlowControl|RetriggerableDelay (Variables|Default|GetFireRate))
                          (goto _label))
                        (:then_2
                          (if (<= (Variables|Default|GetAmmoCount) 0)
                            (CallFunction|StopFire)
                            (CallFunction|SprayStop))))))))
              (else
                (goto _label_2)))
            (else
              (Audio|PlaySoundatLocation "/Game/FPS/FPS_PAWN/DryFire.DryFire" (Transformation|GetWorldLocation (Variables|Default|GetWeapon)) "0, 0, 0" 1.0 1.0 0.0 0 0 0 0))))
        (:then_1
          ;[1 1 1] Bullet Spread
          (if (> (Variables|Default|GetAmmoCount) 0)
            (bind (_direction _bulletspreadvalue) (Timeline|Timeline Play)
              (:Update
                (switch Utilities|FlowControl|Switch|SwitchonETimelineDirection _direction
                  (:Forward
                    (bind _output_get (Variables|Default|SetBulletSpread _bulletspreadvalue)))
                  (:Backward
                    (Variables|Default|SetBulletSpread _bulletspreadvalue)))))))))))

(event Custom|UnEquip
  (params (FPSArmsCharacter :type FPS%20Arms%20Character%20Object%20Reference)))

(event Custom|StopFire
  (bind _character (Variables|Default|GetCharacter))
  (Utilities|FlowControl|Sequence
    (:then_0
      (Utilities|FlowControl|Gate true) ; enters at Close
    )
    (:then_1
      (Variables|/Game/FPS/Blueprints/FPSArms_character.FPSArms_character_C|SetMinRecoil (Variables|Default|GetCharacter) 0.0))
    (:then_2
      ;[1 1 1] Bullet Spread
      (bind (_direction _bulletspreadvalue) (Timeline|Timeline Reverse)
        (:Update
          (switch Utilities|FlowControl|Switch|SwitchonETimelineDirection _direction
            (:Forward
              (bind _output_get (Variables|Default|SetBulletSpread _bulletspreadvalue)))
            (:Backward
              (Variables|Default|SetBulletSpread _bulletspreadvalue))))))))

(event Custom|Equip)

(event Custom|SprayStop)

(event Custom|SprayStart)

(event EventTick
  (params (DeltaSeconds :type Float%20%28single-precision%29))
  (bind _character (Variables|Default|GetCharacter))
  (Utilities|IsValid _character
    (:Is%20Valid
      (Development|PrintString (Utilities|String|ToString(Float) (Variables|/Game/FPS/Blueprints/FPSArms_character.FPSArms_character_C|GetMinRecoil _character)) true true "(R=0.000000,G=0.660000,B=1.000000,A=1.000000)" DeltaSeconds))))

(fn ConstructionScript
  (bind _returnvalue (Utilities|GetDataTableRow "/Game/FPS/Blueprints/Weapons/WeaponTable.WeaponTable" (Utilities|String|StringToName (Variables|Default|GetWeaponEquipped)))
    (:then
      (Variables|Default|SetWeaponName (.WeaponName (Utilities|Struct|BreakWeaponsDetails _returnvalue)))
      (Variables|Default|SetWeaponClass (.Class (Utilities|Struct|BreakWeaponsDetails _returnvalue)))
      (Variables|Default|SetAmmoCount (.AmmoCount (Utilities|Struct|BreakWeaponsDetails _returnvalue)))
      (Variables|Default|SetMaxAmmo (.MaxAmmo (Utilities|Struct|BreakWeaponsDetails _returnvalue)))
      (Variables|Default|SetReloadTime (.ReloadTime (Utilities|Struct|BreakWeaponsDetails _returnvalue)))
      (Variables|Default|SetRecoil (.Recoil (Utilities|Struct|BreakWeaponsDetails _returnvalue)))
      (Variables|Default|SetBulletSpread (.BulletSpread (Utilities|Struct|BreakWeaponsDetails _returnvalue)))
      (Variables|Default|SetFireRate (.FireRate (Utilities|Struct|BreakWeaponsDetails _returnvalue)))
      (Variables|Default|SetAutoFire (.AutoFire (Utilities|Struct|BreakWeaponsDetails _returnvalue)))
      (Variables|Default|SetPickupClass (.PickUpClass (Utilities|Struct|BreakWeaponsDetails _returnvalue)))
      (Variables|Default|SetType (.Type (Utilities|Struct|BreakWeaponsDetails _returnvalue)))
      (Variables|Default|SetAimDS_Anim_Montage (.RifleAimDSAnimMontage (Utilities|Struct|BreakWeaponsDetails _returnvalue)))
      (Variables|Default|SetReload_Anim_Montage (.ReloadAnimation (Utilities|Struct|BreakWeaponsDetails _returnvalue))))))

(fn Shoot
  (params (PlayerController :type Player%20Controller%20Object%20Reference) (PlayeCharacter :type FPS%20Arms%20Character%20Object%20Reference))
  (bind _bulletspread (Variables|Default|GetBulletSpread))
  (bind _character (Variables|Default|GetCharacter))
  (bind _muzzle (Variables|Default|GetMuzzle))
  (bind _returnvalue (Transformation|GetWorldLocation _muzzle))
  (bind _returnvalue_2 (* _bulletspread -1.0))
  (bind _spraypoint (Variables|/Game/FPS/Blueprints/FPSArms_character.FPSArms_character_C|GetSprayPoint _character))
  (bind _returnvalue_3 (Transformation|GetWorldLocation _spraypoint))
  (bind _outhit (Collision|LineTraceByChannel _returnvalue_3 (+ (+ _returnvalue_3 (* (Math|Vector|GetForwardVector _spraypoint) 2e+04)) (Math|Vector|MakeVector (Math|Random|RandomFloatinRange _returnvalue_2 _bulletspread) (Math|Random|RandomFloatinRange _returnvalue_2 _bulletspread) (Math|Random|RandomFloatinRange _returnvalue_2 _bulletspread))) "TraceTypeQuery2" false 0 "None"))
  (bind _asfpsarms_character (Utilities|Casting|CastToFPSArms_character (.HitActor (Collision|BreakHitResult _outhit)))
    (:then
      (if (== (.HitBoneName (Collision|BreakHitResult _outhit)) "Head")
        (Variables|/Game/FPS/Blueprints/FPSArms_character.FPSArms_character_C|SetHealth _asfpsarms_character (- (Variables|/Game/FPS/Blueprints/FPSArms_character.FPSArms_character_C|GetHealth _asfpsarms_character) 1e+02))
        (else
          (Variables|/Game/FPS/Blueprints/FPSArms_character.FPSArms_character_C|SetHealth _asfpsarms_character (- (Variables|/Game/FPS/Blueprints/FPSArms_character.FPSArms_character_C|GetHealth _asfpsarms_character) 1e+01))))
      (if (== (Variables|/Game/FPS/Blueprints/FPSArms_character.FPSArms_character_C|GetHealth _asfpsarms_character) 0.0)
        (Physics|SetSimulatePhysics (Variables|/Script/Engine.Character|GetMesh _asfpsarms_character) true)
        (Class|PrimitiveComponent|SetOwnerNoSee (Variables|/Game/FPS/Blueprints/FPSArms_character.FPSArms_character_C|GetFPSArms _asfpsarms_character) true)
        (Class|PrimitiveComponent|SetOwnerNoSee (Variables|/Script/Engine.Character|GetMesh _asfpsarms_character) false)
        (Input|DisableInput _asfpsarms_character PlayerController)
        (Collision|SetCollisionEnabled (Variables|/Script/Engine.Character|GetCapsuleComponent _asfpsarms_character) "NoCollision")
        (Collision|LineTraceByChannel _returnvalue (.ImpactPoint (Collision|BreakHitResult _outhit)) "TraceTypeQuery1" false 0 "None" true "(R=0.239512,G=0.829331,B=1.000000,A=1.000000)" :!label _label)
        (Game|SpawnActorfromClass "/Game/FPS/Blueprints/Tracer_BP.Tracer_BP_C" (Math|Transform|MakeTransform _returnvalue (Transformation|GetWorldRotation (Variables|/Game/FPS/Blueprints/FPSArms_character.FPSArms_character_C|GetSprayPoint (Variables|Default|GetCharacter))) "0.050000,0.050000,0.050000") "AlwaysSpawn" "OverrideRootScale" 0 0)
        (bind _returnvalue_4 (Game|SpawnActorfromClass "/Game/FPS/Blueprints/Decals_BP.Decals_BP_C" (Math|Transform|MakeTransform (.ImpactPoint (Collision|BreakHitResult _outhit)) (Math|Conversions|RotationFromXVector (.ImpactNormal (Collision|BreakHitResult _outhit))) "0.025000,0.025000,0.025000") "AlwaysSpawn" "OverrideRootScale" 0 0))
        (Rendering|Components|Decal|SetFadeScreenSize (Variables|/Game/FPS/Blueprints/Decals_BP.Decals_BP_C|GetDecal _returnvalue_4) 0.0)
        (bind _returnvalue_5 (Game|SpawnActorfromClass "/Game/FPS/Blueprints/Chaos_Fields/BulletMasterField.BulletMasterField_C" (Math|Transform|MakeTransform (.ImpactPoint (Collision|BreakHitResult _outhit)) "0, 0, 0" "1.000000,1.000000,1.000000") "AlwaysSpawn" "MultiplyWithRoot" 0 0))
        (Variables|Default|SetChaosField _returnvalue_5)
        (Variables|/Game/FPS/Blueprints/Chaos_Fields/BulletMasterField.BulletMasterField_C|SetActivationType (Variables|Default|GetChaosField) "NewEnumerator4")
        (Variables|/Game/FPS/Blueprints/Chaos_Fields/BulletMasterField.BulletMasterField_C|SetFieldLifespan (Variables|Default|GetChaosField) 0.1)
        (Variables|/Game/FPS/Blueprints/Chaos_Fields/BulletMasterField.BulletMasterField_C|SetRadial%20Magnitude (Variables|Default|GetChaosField) 1.5e+02)
        (Default|CETrigger (Variables|Default|GetChaosField))))
    (:CastFailed
      (goto _label))))

(fn AmmoCheck
  (Math|Integer|DecrementInt (Variables|Default|GetAmmoCount)))

(fn AngleBetween2Vectors
  (params (Vector%20A :type Vector) (Vector%20B :type Vector))
  (return (Class|KismetMathLibrary|DegAcos (Math|Vector|DotProduct (Math|Vector|Normalize Vector%20A) (Math|Vector|Normalize Vector%20B)))))