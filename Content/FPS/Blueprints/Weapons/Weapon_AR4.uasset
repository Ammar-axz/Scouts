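; AR4 weapon Blueprint, a child of a shared weapon base, for the first-person character.
; The construction script sets the equipped name before calling the parent; a block setting ammo, automatic fire, timing and pickup class is disconnected.
; AmmoCheck and Shoot overrides do nothing while the player is reloading.
; Otherwise both play the weapon animation and defer to the parent, with AmmoCheck also playing the gunshot sound.
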(fn ConstructionScript
  (Variables|Default|SetWeaponEquipped "AR4")
  (|CallParentFunction))

(fn AmmoCheck
  (if (not (Variables|/Game/FPS/Blueprints/FPSArms_character.FPSArms_character_C|GetIsReloading (.AsFPSArms%20Character (Utilities|Casting|CastToFPSArms_character (Game|GetPlayerCharacter 0)))))
    (Components|Animation|PlayAnimation (Variables|Default|GetWeapon) 0 false)
    (Audio|PlaySoundatLocation "/Game/FPS/FPS_PAWN/Gunshot.Gunshot" (Transformation|GetWorldLocation (Variables|Default|GetWeapon)) "0, 0, 0" 1.0 1.0 0.0 0 0 0 0)
    (|CallParentFunction)))

(fn Shoot
  (params (PlayerController :type Player%20Controller%20Object%20Reference) (PlayeCharacter :type FPS%20Arms%20Character%20Object%20Reference))
  (if (not (Variables|/Game/FPS/Blueprints/FPSArms_character.FPSArms_character_C|GetIsReloading (.AsFPSArms%20Character (Utilities|Casting|CastToFPSArms_character (Game|GetPlayerCharacter 0)))))
    (Components|Animation|PlayAnimation (Variables|Default|GetWeapon) 0 false)
    (|CallParentFunction 0 0)))